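; VR web browser actor whose widget component hosts UMG_WebBrowser and is clicked with the right controller trigger.
; On BeginPlay it takes the VR pawn's right widget interaction component and passes it to the browser widget.
; Trigger press and release become left mouse clicks, with input enabled on overlap or by EnableInputActor and disabled when overlap ends.
; The construction script starts it hidden with collision off.
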(event `InputAction|TriggerRight`
  (params (Key :type "Key Structure"))
  (bind _widget_interaction_right (`self.Widget Interaction Right`))
  ;[0.03434 0.03434 0.03434] Menu Input Right
  (:`Pressed`
    (`WidgetInteractionComponent.PressPointerKey` _widget_interaction_right "LeftMouseButton"))
  (:`Released`
    (`WidgetInteractionComponent.ReleasePointerKey` _widget_interaction_right "LeftMouseButton")))

(event `/Game/VR/Default/BPI_InputSetting.EnableInputActor`
  (params (IsEnable :type Boolean))
  ;[1 1 1] 코멘트
  (`self.EnableInput` (`GameplayStatics.GetPlayerController` 0)))

(event `self.ReceiveBeginPlay`
  ;[1 1 1] 코멘트
  (bind _asvrpawn (cast `/Game/VRTemplate/Blueprints/VRPawn` (`GameplayStatics.GetPlayerPawn` 0)))
  (bind _output_get (set `self.Widget Interaction Right` (`/Game/VRTemplate/Blueprints/VRPawn.WidgetInteractionRight` _asvrpawn)))
  (bind _asumg_web_browser (cast `/Game/VR/Web/UMG_WebBrowser` (`WidgetComponent.GetUserWidgetObject` (`self.Widget`))))
  (set `/Game/VR/Web/UMG_WebBrowser.WidgetInteraction` _output_get _asumg_web_browser))

(event `/Game/VR/Default/BPI_SelectArea.OnBeginOverlap`
  ;[1 1 1] 코멘트
  (`self.EnableInput` (`GameplayStatics.GetPlayerController` 0)))

(event `/Game/VR/Default/BPI_SelectArea.OnEndOverlap`
  ;[1 1 1] 코멘트
  (`self.DisableInput` (`GameplayStatics.GetPlayerController` 0)))

(fn `UserConstructionScript`
  (`SceneComponent.SetVisibility` (`self.Widget`) false false)
  (`self.SetActorEnableCollision` false))