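; VR menu actor that shows a UMG_Menu widget 20 units above a motion controller, turned toward the player camera every Tick.
; On BeginPlay it takes the right widget interaction component from VRPawn and passes it to the menu.
; The right trigger presses and releases a simulated left mouse click through that component.
; Overlap begin and end toggle the actor's input, and EnableInputActor can also enable it.
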(event `InputAction|TriggerRight`
  (params (Key :type "Key Structure"))
  (bind _widget_interaction_right (`self.Widget Interaction Right`))
  ;[0.03434 0.03434 0.03434] Menu Input Right
  (:`Pressed`
    (`WidgetInteractionComponent.PressPointerKey` _widget_interaction_right "LeftMouseButton"))
  (:`Released`
    (`WidgetInteractionComponent.ReleasePointerKey` _widget_interaction_right "LeftMouseButton")))

(event `self.ReceiveTick`
  (params (DeltaSeconds :type "Float (single-precision)"))
  ;[1 1 1] 코멘트
  (`SceneComponent.K2_SetWorldLocation` (`self.MenuWidget`) (+ (`SceneComponent.K2_GetComponentLocation` (`self.MotionController`)) (0.0 0.0 20.0)) false false)
  (`SceneComponent.K2_SetWorldRotation` (`self.MenuWidget`) (`KismetMathLibrary.FindLookAtRotation` (`SceneComponent.K2_GetComponentLocation` (`self.MenuWidget`)) (`self.K2_GetActorLocation` (`GameplayStatics.GetPlayerCameraManager` 0))) false false))

(event `/Game/VR/Default/BPI_InputSetting.EnableInputActor`
  (params (IsEnable :type Boolean))
  ;[1 1 1] 코멘트
  (`self.EnableInput` (`GameplayStatics.GetPlayerController` 0)))

(event `self.ReceiveBeginPlay`
  ;[1 1 1] 코멘트
  (bind _asvrpawn (cast `/Game/VRTemplate/Blueprints/VRPawn` (`GameplayStatics.GetPlayerPawn` 0)))
  (bind _output_get (set `self.Widget Interaction Right` (`/Game/VRTemplate/Blueprints/VRPawn.WidgetInteractionRight` _asvrpawn)))
  (bind _asumg_menu (cast `/Game/VR/Default/UMG_Menu` (`WidgetComponent.GetUserWidgetObject` (`self.MenuWidget`))))
  (set `/Game/VR/Default/UMG_Menu.WidgetInteraction` _output_get _asumg_menu))

(event `/Game/VR/Default/BPI_SelectArea.OnBeginOverlap`
  ;[1 1 1] 코멘트
  (`self.EnableInput` (`GameplayStatics.GetPlayerController` 0)))

(event `/Game/VR/Default/BPI_SelectArea.OnEndOverlap`
  ;[1 1 1] 코멘트
  (`self.DisableInput` (`GameplayStatics.GetPlayerController` 0)))

(fn `UserConstructionScript`)